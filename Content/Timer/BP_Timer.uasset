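; BP_Timer is a simple timer Blueprint that counts elapsed minutes and seconds.
; Tick drives a one-second Delay, which ignores calls while pending, so Second increments roughly once per second and can drift with frame timing.
; When Second reaches 60, it resets to zero and Minutes increments.
; The Blueprint only updates these variables, with no display, stop or reset logic.
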(event `self.ReceiveTick`
  (params (DeltaSeconds :type "Float (single-precision)"))
  (`KismetSystemLibrary.Delay` 1.0)
  (set `self.Second` (+ (`self.Second`) 1))
  (if (>= (`self.Second`) 60)
    (set `self.Minutes` (+ (`self.Minutes`) 1))
    (set `self.Second` 0)))

(fn `UserConstructionScript`)