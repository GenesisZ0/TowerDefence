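; BP_Enemie1 is a tower defense enemy, an orc that walks along a spline path.
; A Timeline, with play rate derived from Speed, drives location and tangent-based rotation from spline start to last point.
; Reaching the end reduces player life through the HUD and destroys the enemy.
; DicreaseLife applies damage; on death it awards gold, gives experience to the attacking tower, updates that tower's widget and destroys the actor.
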(event `self.ReceiveBeginPlay`
  (bind _spline (`/Game/Spline_Mouvement/spline_mouvement.Spline` (`self.Spline`)))
  (`|ExecutionSequence`
    (:`then_0`
      (bind _outactors (`GameplayStatics.GetAllActorsOfClass` "/Game/Spawner/BP_EnemierSpawner.BP_EnemierSpawner_C"))
      (set `self.Spawner` _outactors)
      (bind _returnvalue (`GameplayStatics.GetActorOfClass` "/Game/Player/PlayerController2.PlayerController2_C"))
      (set `self.PlayerCrEF` _returnvalue)
      (bind _returnvalue_2 (`GameplayStatics.GetActorOfClass` "/Game/Battiment/Tower/BP_Tower.BP_Tower_C"))
      (set `self.TowerRef` _returnvalue_2))
    (:`then_1`
      (`PrimitiveComponent.SetCollisionResponseToChannel` (`self.SkeletalMesh`) "ECC_Visibility" "ECR_Ignore"))
    (:`then_2`
      (`KismetSystemLibrary.Delay` 0.2)
      (`TimelineComponent.SetPlayRate` (`self.Timeline`) (/ 1.0 (`self.Speed`)))
      (`SkeletalMeshComponent.PlayAnimation` (`self.SkeletalMesh`) "/Game/Animation/Orc_Walk__1_.Orc_Walk__1_" true)
      (bind (_direction _newtrack_0) (`Timeline|Timeline` :!via `PlayFromStart`)
        (:`Update`
          (bind _returnvalue_3 (`KismetMathLibrary.Lerp` 0.0 (`SplineComponent.GetDistanceAlongSplineAtSplinePoint` _spline (- (`SplineComponent.GetNumberOfSplinePoints` _spline) 1)) _newtrack_0))
          (`self.K2_SetActorLocation` (`SplineComponent.GetLocationAtDistanceAlongSpline` _spline _returnvalue_3 "World"))
          (`self.K2_SetActorRotation` (`KismetMathLibrary.Conv_VectorToRotator` (`SplineComponent.GetTangentAtDistanceAlongSpline` _spline _returnvalue_3 "Local"))))
        (:`Finished`
          (`/Game/Player/BP_HUD.ReduceLife` (`/Game/Player/PlayerController2.BP_HUD` (`self.PlayerCrEF`)) (`self.Dammage`))
          (`self.K2_DestroyActor`))))))

(event `DicreaseLife`
  (params (Damage :type "Float (double-precision)") (TowerMother :type "/Game/Battiment/Tower/BP_Tower Object Reference"))
  (bind _playercref (`self.PlayerCrEF`))
  (set `self.Health` (- (`self.Health`) Damage))
  (if (<= (`self.Health`) 0.0)
    (set `/Game/Player/PlayerController2.Gold` (+ (`/Game/Player/PlayerController2.Gold` _playercref) 25) _playercref)
    (bind _asbp_exptower_hud (cast `/Game/BP_ExptowerHud` (`WidgetComponent.GetWidget` (`/Game/Battiment/Tower/BP_Tower.Widget` TowerMother))))
    (set `self.As BP Exptower Hud` _asbp_exptower_hud)
    (set `/Game/Battiment/Tower/BP_Tower.ExpActu` (+ (`self.ExpGiven`) (`/Game/Battiment/Tower/BP_Tower.ExpActu` TowerMother)) TowerMother)
    (`/Game/BP_ExptowerHud.GetExp` (`self.As BP Exptower Hud`) TowerMother)
    (`self.K2_DestroyActor`)))

(fn `UserConstructionScript`)