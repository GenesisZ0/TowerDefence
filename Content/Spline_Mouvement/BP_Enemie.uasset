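; BP_Enemie is an enemy that walks along a spline path and damages the player's life on reaching the end.
; After a short delay, it loops an orc walk animation and starts a timeline with play rate 1/Speed, so Speed acts as travel duration.
; The timeline lerps distance along the spline to set location and tangent-facing rotation.
; On finish, it calls ReduceLife on the player controller's HUD and destroys itself.
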(event `self.ReceiveBeginPlay`
  (bind _spline (`/Game/Spline_Mouvement/spline_mouvement.Spline` (`self.Spline`)))
  (`|ExecutionSequence`
    (:`then_0`
      (bind _outactors (`GameplayStatics.GetAllActorsOfClass` "/Game/Spawner/BP_EnemierSpawner.BP_EnemierSpawner_C"))
      (set `self.Spawner` _outactors)
      (bind _returnvalue (`GameplayStatics.GetActorOfClass` "/Game/Player/PlayerController2.PlayerController2_C"))
      (set `self.PlayerCrEF` _returnvalue))
    (:`then_1`
      (`PrimitiveComponent.SetCollisionResponseToChannel` (`self.SkeletalMesh`) "ECC_Visibility" "ECR_Ignore"))
    (:`then_2`
      (`KismetSystemLibrary.Delay` 0.2)
      (`TimelineComponent.SetPlayRate` (`self.Timeline`) (/ 1.0 (`self.Speed`)))
      (`SkeletalMeshComponent.PlayAnimation` (`self.SkeletalMesh`) "/Game/Animation/Orc_Walk__1_.Orc_Walk__1_" true)
      (bind (_direction _newtrack_0) (`Timeline|Timeline` :!via `PlayFromStart`)
        (:`Update`
          (bind _returnvalue_2 (`KismetMathLibrary.Lerp` 0.0 (`SplineComponent.GetDistanceAlongSplineAtSplinePoint` _spline (- (`SplineComponent.GetNumberOfSplinePoints` _spline) 1)) _newtrack_0))
          (`self.K2_SetActorLocation` (`SplineComponent.GetLocationAtDistanceAlongSpline` _spline _returnvalue_2 "World"))
          (`self.K2_SetActorRotation` (`KismetMathLibrary.Conv_VectorToRotator` (`SplineComponent.GetTangentAtDistanceAlongSpline` _spline _returnvalue_2 "Local"))))
        (:`Finished`
          (`/Game/Player/BP_HUD.ReduceLife` (`/Game/Player/PlayerController2.BP_HUD` (`self.PlayerCrEF`)) (`self.Dammage`))
          (`self.K2_DestroyActor`))))))

(fn `UserConstructionScript`)