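; BP_EnemierSpawner is an enemy spawner that repeatedly spawns actors at its Sphere component's location.
; Tick calls SpawnEnemie, whose latent Delay paces the spawning.
; Each spawn cast to BP_Enemie1 receives the spawner's Spline and current Speed.
; It then raises Speed and shortens Delay whenever BP_Timer's Minutes plus one is nonzero, so difficulty ramps per spawn rather than per minute.
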(event `self.ReceiveBeginPlay`
  (bind _returnvalue (`GameplayStatics.GetActorOfClass` "/Game/Timer/BP_Timer.BP_Timer_C"))
  (set `self.Timer` _returnvalue))

(event `self.ReceiveTick`
  (params (DeltaSeconds :type "Float (single-precision)"))
  (`self.SpawnEnemie` (`self.Delay`) (`KismetMathLibrary.MakeTransform` (`SceneComponent.K2_GetComponentLocation` (`self.Sphere`)))))

(event `SpawnEnemie`
  (params (Delay :type "Float (double-precision)") (location :type "Transform Structure"))
  (`KismetSystemLibrary.Delay` Delay)
  (bind _returnvalue (`|SpawnActorFromClass` (`self.Actor`) location "Undefined" "OverrideRootScale" null null))
  (bind _asbp_enemie_1 (cast `/Game/Spline_Mouvement/BP_Enemie1` _returnvalue))
  (set `/Game/Spline_Mouvement/BP_Enemie1.Spline` (`self.Spline`) _asbp_enemie_1)
  (set `self.EnemieSpawnRef` _asbp_enemie_1)
  (set `/Game/Spline_Mouvement/BP_Enemie1.Speed` (`self.Speed`) _asbp_enemie_1)
  (if (`KismetMathLibrary.Conv_IntToBool` (+ (`/Game/Timer/BP_Timer.Minutes` (`self.Timer`)) 1))
    (set `self.Speed` (+ (`self.Speed`) 0.2))
    (set `self.Delay` (- (`self.Delay`) 0.1))))

(fn `UserConstructionScript`)