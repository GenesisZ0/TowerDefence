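; BP_Projo is a tower projectile that homes in on a target and damages enemies on contact.
; The Homming event checks that the target is valid, then sets it as the ProjectileMovement homing component with a high homing acceleration.
; When its Sphere overlaps a BP_Enemie1, it passes Damage to DicreaseLife and destroys itself, ignoring other actors.
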(event `self.ReceiveBeginPlay`
  (`|ExecutionSequence`))

(event `Homming`
  (params (Target :type "StaticMeshComponent Object Reference"))
  (bind _projectilemovement (`self.ProjectileMovement`))
  (if (`KismetSystemLibrary.IsValid` Target)
    (set `ProjectileMovementComponent.HomingTargetComponent` Target _projectilemovement)
    (set `ProjectileMovementComponent.bIsHomingProjectile` true _projectilemovement)
    (set `ProjectileMovementComponent.HomingAccelerationMagnitude` 25000.0 _projectilemovement)))

(event `self.Sphere.OnComponentBeginOverlap`
  (params (OverlappedComponent :type "PrimitiveComponent Object Reference") (OtherActor :type "Actor Object Reference") (OtherComp :type "PrimitiveComponent Object Reference") (OtherBodyIndex :type Integer) (bFromSweep :type Boolean) (SweepResult :type "HitResult Structure (by ref)"))
  (bind _asbp_enemie_1 (cast `/Game/Spline_Mouvement/BP_Enemie1` OtherActor))
  (`/Game/Spline_Mouvement/BP_Enemie1.DicreaseLife` _asbp_enemie_1 (`self.Damage`))
  (`self.K2_DestroyActor`))

(fn `UserConstructionScript`)